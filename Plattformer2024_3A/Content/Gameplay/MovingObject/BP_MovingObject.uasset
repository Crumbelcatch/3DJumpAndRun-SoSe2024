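; BP_MovingObject is a triggerable actor whose mesh moves between its start location and a TargetLocation point.
; A trigger either moves it immediately or starts a delay timer and shows a global countdown through the game mode.
; A timeline drives the position lerp, playing forward or reversing based on whether the object has reached the target.
; A resettable DoOnce blocks further moves once a trigger-once object is at its target.
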(event `self.ReceiveBeginPlay`
  ;[0.5613 1 0.3902] Begin play
  (set `self.ObjectStartLocation` (`SceneComponent.K2_GetComponentLocation` (`self.Mesh`)))
  (`TimelineComponent.SetPlayRate` (`self.ObjectMoveAlpha`) (`self.ObjectMoveRate`)))

(event `/Game/Gameplay/Trigger/BPI_TriggerReceiver.TriggerReceiver`
  (params (bTriggersOnce :type Boolean))
  ;[1 1 1] Triggered
  (set `self.CurrentlyTriggersOnce` bTriggersOnce)
  (if (> (`self.MoveDelayedBy`) 0.0)
    (`KismetSystemLibrary.K2_SetTimerDelegate` (`|CreateDelegate` :!event `TriggerObjectMove`) (`self.MoveDelayedBy`))
    (message `/Game/Core/BPI_GameMode.ShowHideGlobalCountdown` (`GameplayStatics.GetGameMode`) (`self.MoveDelayedBy`) true)
    (else
      (`self.TriggerObjectMove`))))

(event `TriggerObjectMove`
  ;[1 1 1] Object Move
  (`|ExecutionSequence`
    (:`then_0`
      (if (or (not (`self.CurrentlyTriggersOnce`)) (and (`self.CurrentlyTriggersOnce`) (not (`self.bObjectAtTargetLocation`))))
        (`self.ResetMovementDoOnce`)))
    (:`then_1`
      (`/Engine/EditorBlueprintResources/StandardMacros.DoOnce` false :!label _label
        (:`Completed`
          (if (not (`self.bObjectAtTargetLocation`))
            (bind (_direction _alpha_0_1) (`Timeline|ObjectMoveAlpha` :!label _label_2)
              (:`Update`
                (`SceneComponent.K2_SetWorldLocation` (`self.Mesh`) (`KismetMathLibrary.VLerp` (`self.ObjectStartLocation`) (`SceneComponent.K2_GetComponentLocation` (`self.TargetLocation`)) _alpha_0_1) false false))
              (:`Finished`
                ;[1 1 1] Object move finished
                (switch `ETimelineDirection` _direction
                  (:`Forward`
                    (set `self.bObjectAtTargetLocation` true))
                  (:`Backward`
                    (set `self.bObjectAtTargetLocation` false)))))
            (else
              (goto _label_2 :!via `Reverse`))))))))

(event `ResetMovementDoOnce`
  ;[1 1 1] Object Move
  (goto _label :!via `Reset`))

(fn `UserConstructionScript`)