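; Triggerable actor that moves an object along a spline, starting from the spline's beginning.
; A trigger interface event starts a looping timer that advances distance by Speed and delta seconds.
; At either end it wraps on closed looping splines, ping-pongs on open looping ones, or stops and reverses for the next trigger.
; A DoOnce blocks retriggering, resetting only for repeatable triggers once a non-looping move has stopped.
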(event `self.ReceiveBeginPlay`
  ;[0.5626 1 0.4205] Begin play
  (`SceneComponent.K2_SetWorldLocation` (`self.MovingObject`) (`SplineComponent.GetLocationAtDistanceAlongSpline` (`self.Spline`) 0.0 "World") false false)
  (set `self.CurrentDistance` 0.0)
  (set `self.bMovingForward` true))

(event `/Game/Gameplay/Trigger/BPI_TriggerReceiver.TriggerReceiver`
  (params (bTriggersOnce :type Boolean))
  ;[1 1 1] Trigger from interface
  (set `self.CurrentlyTriggersOnce` bTriggersOnce)
  (`|ExecutionSequence`
    (:`then_0`
      (if (and (not (`self.CurrentlyTriggersOnce`)) (or (>= (`self.CurrentDistance`) (`SplineComponent.GetSplineLength` (`self.Spline`))) (== (`self.CurrentDistance`) 0.0)) (and (not (`self.bLoopOnSpline`)) (not (`KismetSystemLibrary.K2_IsTimerActiveHandle` (`self.ObjectMovementTimer`)))))
        (`self.ResetMovementDoOnce`)))
    (:`then_1`
      (`/Engine/EditorBlueprintResources/StandardMacros.DoOnce` false :!label _label
        (:`Completed`
          (`self.StartMoving`))))))

(event `ResetMovementDoOnce`
  ;[1 1 1] Trigger from interface
  (goto _label :!via `Reset`))

(event `StartMoving`
  ;[1 1 1] Start Moving
  (bind _returnvalue (`KismetSystemLibrary.K2_SetTimerDelegate` (delegate `MoveObject`) 0.01 true))
  (set `self.ObjectMovementTimer` _returnvalue))

(event `MoveObject`
  ;[1 1 1] Move object update
  (if (or (and (< (`self.CurrentDistance`) (`SplineComponent.GetSplineLength` (`self.Spline`))) (`self.bMovingForward`)) (and (> (`self.CurrentDistance`) 0.0) (not (`self.bMovingForward`))))
    (bind _newdistance (`self.CalculateDistance` (`self.bMovingForward`)))
    (bind _output_get (set `self.CurrentDistance` _newdistance))
    (`SceneComponent.K2_SetWorldLocation` (`self.MovingObject`) (`SplineComponent.GetLocationAtDistanceAlongSpline` (`self.Spline`) _output_get "World") false false)
    (else
      ;[1 1 1] Looping movement
      (if (and (`SplineComponent.IsClosedLoop` (`self.Spline`)) (`self.bLoopOnSpline`))
        (set `self.CurrentDistance` 0.0)
        (elif (`self.bLoopOnSpline`)
          (`/Engine/EditorBlueprintResources/StandardMacros.FlipFlop`
            (:`A`
              (set `self.bMovingForward` false)
              (set `self.CurrentDistance` (`SplineComponent.GetSplineLength` (`self.Spline`))))
            (:`B`
              (set `self.bMovingForward` true)
              (set `self.CurrentDistance` 0.0)))
          (else
            ;[1 0.4456 0.1437] Stop movement
            (`KismetSystemLibrary.K2_ClearAndInvalidateTimerHandle` (`self.ObjectMovementTimer`))
            (`/Engine/EditorBlueprintResources/StandardMacros.FlipFlop`
              (:`A`
                (set `self.bMovingForward` false)
                (set `self.CurrentDistance` (`SplineComponent.GetSplineLength` (`self.Spline`))))
              (:`B`
                (set `self.bMovingForward` true)
                (set `self.CurrentDistance` 0.0)))))))))

(fn `CalculateDistance`
  (params (bMovingForward :type Boolean))
  (returns (NewDistance :type "Float (double-precision)"))
  (if bMovingForward
    (return (+ (`self.CurrentDistance`) (* (`self.Speed`) (`GameplayStatics.GetWorldDeltaSeconds`))))
    (else
      (return (- (`self.CurrentDistance`) (* (`self.Speed`) (`GameplayStatics.GetWorldDeltaSeconds`)))))))

(fn `UserConstructionScript`)