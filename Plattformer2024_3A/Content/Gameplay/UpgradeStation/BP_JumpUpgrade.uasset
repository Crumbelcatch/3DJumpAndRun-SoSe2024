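; BP_JumpUpgrade is a jump upgrade pickup that shows tutorial text when collected.
; On overlap with a Player-tagged actor, it flags the upgrade as collected on player character 0 and has the game mode show its tutorial textbox.
; It then hides the sphere and disables collision instead of destroying itself, clearing the textbox after a five-second delay.
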(event `self.Collision.OnComponentBeginOverlap`
  (params (OverlappedComponent :type "PrimitiveComponent Object Reference") (OtherActor :type "Actor Object Reference") (OtherComp :type "PrimitiveComponent Object Reference") (OtherBodyIndex :type Integer) (bFromSweep :type Boolean) (SweepResult :type "HitResult Structure (by ref)"))
  (if (`self.ActorHasTag` OtherActor "Player")
    (message `/Game/Characters/Player/BPI_Upgrades.SetJumpUpCollected` (`GameplayStatics.GetPlayerCharacter` 0) true)
    (message `/Game/Core/BPI_GameMode.ShowHideTutorialTextbox` (`GameplayStatics.GetGameMode`) (`self.TutorialTextTitle`) (`self.TutorialText`) true)
    (`SceneComponent.SetHiddenInGame` (`self.Sphere`) true true)
    (`PrimitiveComponent.SetCollisionEnabled` (`self.Collision`) "NoCollision")
    (`KismetSystemLibrary.Delay` 5.0)
    (message `/Game/Core/BPI_GameMode.ShowHideTutorialTextbox` (`GameplayStatics.GetGameMode`) "" "" false)))

(fn `UserConstructionScript`)