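; Upgrade station that unlocks the player's jump and umbrella upgrades when the player overlaps its collision.
; Each upgrade is checked in turn through player character messages and is granted only if collected and not yet upgraded.
; Granting one sets the upgraded state, plays an unlock sound at the station and shows a tutorial textbox through the game mode, hidden again after a short delay.
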(event `self.Collision.OnComponentBeginOverlap`
  (params (OverlappedComponent :type "PrimitiveComponent Object Reference") (OtherActor :type "Actor Object Reference") (OtherComp :type "PrimitiveComponent Object Reference") (OtherBodyIndex :type Integer) (bFromSweep :type Boolean) (SweepResult :type "HitResult Structure (by ref)"))
  (if (`self.ActorHasTag` OtherActor "Player")
    (`|ExecutionSequence`
      (:`then_0`
        ;[1 1 1] Jump Upgrade
        (bind _bjumpupgraded (message `/Game/Characters/Player/BPI_Upgrades.GetJumpUpgraded` (`GameplayStatics.GetPlayerCharacter` 0)))
        (if (not _bjumpupgraded)
          (bind _bjumpupcollected (message `/Game/Characters/Player/BPI_Upgrades.GetJumpUpCollected` (`GameplayStatics.GetPlayerCharacter` 0)))
          (if _bjumpupcollected
            (bind _return (message `/Game/Characters/Player/BPI_Upgrades.SetJumpUpgraded` (`GameplayStatics.GetPlayerCharacter` 0) _bjumpupcollected))
            (`FMODBlueprintStatics.PlayEventAtLocation` "/Game/FMOD/Events/Environment/SFX_Upgrade_Unlock.SFX_Upgrade_Unlock" (`KismetMathLibrary.MakeTransform` (`SceneComponent.K2_GetComponentLocation` (`self.Collision`))))
            (message `/Game/Core/BPI_GameMode.ShowHideTutorialTextbox` (`GameplayStatics.GetGameMode`) (`self.UpgradeHeader`) (`self.JumpUpgradedTutorial`) _return)
            (`KismetSystemLibrary.Delay` 5.0)
            (message `/Game/Core/BPI_GameMode.ShowHideTutorialTextbox` (`GameplayStatics.GetGameMode`) "" "" false))))
      (:`then_1`
        ;[1 1 1] Umbrella Upgrade
        (bind _bumbrellaupgraded (message `/Game/Characters/Player/BPI_Upgrades.GetUmbrellaUpgraded` (`GameplayStatics.GetPlayerCharacter` 0)))
        (if (not _bumbrellaupgraded)
          (bind _bupgradecollected (message `/Game/Characters/Player/BPI_Upgrades.GetUmbrellaUpCollected` (`GameplayStatics.GetPlayerCharacter` 0)))
          (if _bupgradecollected
            (bind _return_2 (message `/Game/Characters/Player/BPI_Upgrades.SetUmbrellaUpgraded` (`GameplayStatics.GetPlayerCharacter` 0) true))
            (`FMODBlueprintStatics.PlayEventAtLocation` "/Game/FMOD/Events/Environment/SFX_Upgrade_Unlock.SFX_Upgrade_Unlock" (`KismetMathLibrary.MakeTransform` (`SceneComponent.K2_GetComponentLocation` (`self.Collision`))))
            (message `/Game/Core/BPI_GameMode.ShowHideTutorialTextbox` (`GameplayStatics.GetGameMode`) (`self.UpgradeHeader`) (`self.UmbrellaUpgradedTutorial`) _return_2)
            (`KismetSystemLibrary.Delay` 5.0)
            (message `/Game/Core/BPI_GameMode.ShowHideTutorialTextbox` (`GameplayStatics.GetGameMode`) "" "" false)))))))

(fn `UserConstructionScript`)