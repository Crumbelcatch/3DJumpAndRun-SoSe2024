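; BP_UmbrellaUpgrade is a pickup that grants the player the umbrella upgrade and shows a tutorial message.
; When an actor tagged Player overlaps its collision, it sends SetUmbrellaUpCollectedMessage to the player character.
; If that returns true, it hides the sphere and disables collision so it cannot retrigger.
; It then has the game mode show the tutorial textbox, hiding it after a short delay.
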(event `self.Collision.OnComponentBeginOverlap`
  (params (OverlappedComponent :type "PrimitiveComponent Object Reference") (OtherActor :type "Actor Object Reference") (OtherComp :type "PrimitiveComponent Object Reference") (OtherBodyIndex :type Integer) (bFromSweep :type Boolean) (SweepResult :type "HitResult Structure (by ref)"))
  (if (`self.ActorHasTag` OtherActor "Player")
    (bind _return (message `/Game/Characters/Player/BPI_Upgrades.SetUmbrellaUpCollected` (`GameplayStatics.GetPlayerCharacter` 0) true))
    (if _return
      (`SceneComponent.SetHiddenInGame` (`self.Sphere`) true true)
      (`PrimitiveComponent.SetCollisionEnabled` (`self.Collision`) "NoCollision")
      (message `/Game/Core/BPI_GameMode.ShowHideTutorialTextbox` (`GameplayStatics.GetGameMode`) (`self.TutorialTextContent`) true)
      (`KismetSystemLibrary.Delay` 5.0)
      (message `/Game/Core/BPI_GameMode.ShowHideTutorialTextbox` (`GameplayStatics.GetGameMode`) (`self.TutorialTextContent`) false))))

(fn `UserConstructionScript`)