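; Simple spinning collectable that the player picks up by overlapping it.
; On BeginPlay it registers itself with the game mode through a message call and sets a random yaw spin speed.
; An overlap by a Player-tagged actor notifies the game mode, then ToggleCollectable hides the mesh and disables collision.
; The actor is never destroyed, and the same toggle can show it and restore query-only collision.
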(event `self.ReceiveBeginPlay`
  ;[0.4216 1 0.3943] Begin play
  (message `/Game/Gameplay/Collectables/BPI_Collectables.RegisterNewCollectable` (`GameplayStatics.GetGameMode`) self)
  (set `RotatingMovementComponent.RotationRate` (`KismetMathLibrary.MakeRotator` 0.0 0.0 (`KismetMathLibrary.RandomFloatInRange` 100.0 180.0)) (`self.RotatingMovement`)))

(event `self.Collision.OnComponentBeginOverlap`
  (params (OverlappedComponent :type "PrimitiveComponent Object Reference") (OtherActor :type "Actor Object Reference") (OtherComp :type "PrimitiveComponent Object Reference") (OtherBodyIndex :type Integer) (bFromSweep :type Boolean) (SweepResult :type "HitResult Structure (by ref)"))
  ;[1 1 1] Begin overlap
  (if (`self.ActorHasTag` OtherActor "Player")
    (message `/Game/Gameplay/Collectables/BPI_Collectables.Collected` (`GameplayStatics.GetGameMode`) self)
    (`self.ToggleCollectable` false)))

(event `ToggleCollectable`
  (params (bActive :type Boolean))
  ;[1 1 1] Toggle collectable
  (if bActive
    (`SceneComponent.SetHiddenInGame` (`self.CollectableMesh`) false false)
    (`PrimitiveComponent.SetCollisionEnabled` (`self.Collision`) "QueryOnly")
    (else
      (`SceneComponent.SetHiddenInGame` (`self.CollectableMesh`) true false)
      (`PrimitiveComponent.SetCollisionEnabled` (`self.Collision`) "NoCollision"))))

(fn `UserConstructionScript`)