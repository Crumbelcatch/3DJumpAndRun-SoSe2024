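; Overlap trigger actor that fires linked receivers when a player-tagged actor enters its collision, optionally gated by a collectable count.
; It queries the game mode for collected collectables and proceeds when the threshold is zero or met.
; Each referenced receiver gets a BPI_TriggerReceiver interface message carrying a trigger-once flag.
; Invalid receivers or ones lacking the interface print a debug message instead.
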(event `self.Collision.OnComponentBeginOverlap`
  (params (OverlappedComponent :type "PrimitiveComponent Object Reference") (OtherActor :type "Actor Object Reference") (OtherComp :type "PrimitiveComponent Object Reference") (OtherBodyIndex :type Integer) (bFromSweep :type Boolean) (SweepResult :type "HitResult Structure (by ref)"))
  ;[1 1 1] Begin overlap
  (if (`self.ActorHasTag` OtherActor "Player")
    (bind _collectedcollectables (message `/Game/Gameplay/Collectables/BPI_Collectables.GetCollectedCollectables` (`GameplayStatics.GetGameMode`)))
    (if (or (== (`self.CollectableThreshold`) 0) (>= _collectedcollectables (`self.CollectableThreshold`)))
      (for _array_element (`self.ReceiverRef`)
        (`self.TryTriggerSingleReceiver` _array_element)))))

(fn `TryTriggerSingleReceiver`
  (params (Receiver :type "Actor Object Reference"))
  (locals (LReceiver :type "Actor Object Reference"))
  (bind _lreceiver (`local.LReceiver`))
  (set `local.LReceiver` Receiver)
  (`|ExecutionSequence`
    (:`then_0`
      (`/Engine/EditorBlueprintResources/StandardMacros.IsValid` (`local.LReceiver`)
        (:`Is Valid`
          (if (`KismetSystemLibrary.DoesImplementInterface` _lreceiver "/Game/Gameplay/Trigger/BPI_TriggerReceiver.BPI_TriggerReceiver_C")
            (message `/Game/Gameplay/Trigger/BPI_TriggerReceiver.TriggerReceiver` _lreceiver (`self.TriggersReceiverOnce`))
            (else
              (`KismetSystemLibrary.PrintString` (`KismetStringLibrary.Concat_StrStr` (`KismetSystemLibrary.GetDisplayName` self) " tried to trigger " (`KismetSystemLibrary.GetDisplayName` (`local.LReceiver`)) " but it doesn't implement the interface")))))
        (:`Is Not Valid`
          (`KismetSystemLibrary.PrintString` (`KismetStringLibrary.Concat_StrStr` "Receiver in " (`KismetSystemLibrary.GetDisplayName` self) " is not valid")))))
    (:`then_1`
      (return))))

(fn `UserConstructionScript`)