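; Launch pad actor that launches a Player-tagged actor along the mesh's up vector at a set strength.
; Launching happens on collision overlap only if the player's movement mode is Falling, so walking onto it does nothing.
; Movement component lookup and launch both go through interface messages.
; With ActivatedByTrigger set, it starts hidden without collision until TriggerReceiver reveals and enables it.
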(event `self.ReceiveBeginPlay`
  ;[0.372 1 0.3197] Begin play
  (if (`self.bActivatedByTrigger`)
    (`SceneComponent.SetHiddenInGame` (`self.Mesh`) true false)
    (`PrimitiveComponent.SetCollisionEnabled` (`self.Mesh`) "NoCollision")
    (`PrimitiveComponent.SetCollisionEnabled` (`self.Collision`) "NoCollision")))

(event `/Game/Gameplay/Trigger/BPI_TriggerReceiver.TriggerReceiver`
  (params (bTriggersOnce :type Boolean))
  ;[1 1 1] Trigger
  (switch `ECollisionEnabled` (`PrimitiveComponent.GetCollisionEnabled` (`self.Collision`))
    (:`NoCollision`
      (`SceneComponent.SetHiddenInGame` (`self.Mesh`) false false)
      (`PrimitiveComponent.SetCollisionEnabled` (`self.Mesh`) "QueryAndPhysics")
      (`PrimitiveComponent.SetCollisionEnabled` (`self.Collision`) "QueryOnly"))))

(event `self.Collision.OnComponentBeginOverlap`
  (params (OverlappedComponent :type "PrimitiveComponent Object Reference") (OtherActor :type "Actor Object Reference") (OtherComp :type "PrimitiveComponent Object Reference") (OtherBodyIndex :type Integer) (bFromSweep :type Boolean) (SweepResult :type "HitResult Structure (by ref)"))
  ;[1 1 1] Begin overlap
  (if (`self.ActorHasTag` OtherActor "Player")
    (bind _movementcomponentref (message `/Game/Characters/Player/BPI_PlayerValues.GetCharacterMovementComponent` OtherActor))
    (switch `EMovementMode` (`CharacterMovementComponent.MovementMode` _movementcomponentref)
      (:`MOVE_Falling`
        (message `/Game/Characters/Player/BPI_PlayerManipulation.LaunchPlayer` OtherActor (`SceneComponent.GetUpVector` (`self.Mesh`)) (`self.LaunchStrength`))))))

(fn `UserConstructionScript`)