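; BP_SoundManager is an FMOD audio manager that controls volume levels and background music switching.
; Setters store master, music and SFX volumes and apply them to the Master, Atmo and SFX VCAs, with matching getters.
; SwitchBGM stops and releases any valid current atmo instance, plays the new event in 2D, keeps its handle and prints a debug message.
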(fn `GetMasterVolume`
  (returns (CurrentVolume :type "Float (double-precision)"))
  (return (`self.MasterVolume`)))

(fn `GetMusicVolume`
  (returns (CurrentVolume :type "Float (double-precision)"))
  (return (`self.CurrentMusicVolume`)))

(fn `GetSFXVolume`
  (returns (CurrentVolume :type "Float (double-precision)"))
  (return (`self.CurrentSFXVolume`)))

(fn `SetMasterVolume`
  (params (NewVolume :type "Float (double-precision)"))
  (returns (return :type Boolean))
  (bind _output_get (set `self.MasterVolume` NewVolume))
  (`FMODBlueprintStatics.VCASetVolume` "/Game/FMOD/VCAs/Master.Master" _output_get)
  (return false))

(fn `SetMusicVolume`
  (params (NewVolume :type "Float (double-precision)"))
  (returns (return :type Boolean))
  (bind _output_get (set `self.CurrentMusicVolume` NewVolume))
  (`FMODBlueprintStatics.VCASetVolume` "/Game/FMOD/VCAs/Atmo.Atmo" _output_get)
  (return false))

(fn `SetSFXVolume`
  (params (NewVolume :type "Float (double-precision)"))
  (returns (return :type Boolean))
  (bind _output_get (set `self.CurrentSFXVolume` NewVolume))
  (`FMODBlueprintStatics.VCASetVolume` "/Game/FMOD/VCAs/SFX.SFX" _output_get)
  (return false))

(fn `SwitchBGM`
  (params (NewMusic :type "FMODEvent Object Reference"))
  (returns (Return :type Boolean))
  (locals (LNewBGM :type "FMODEvent Object Reference"))
  (set `local.LNewBGM` NewMusic)
  (bind _returnvalue (`FMODBlueprintStatics.EventInstanceIsValid` (`self.CurrentAtmo`)))
  (if _returnvalue
    (`FMODBlueprintStatics.EventInstanceStop` (`self.CurrentAtmo`) true))
  (bind _returnvalue_2 (`FMODBlueprintStatics.PlayEvent2D` (`local.LNewBGM`)))
  (set `self.CurrentAtmo` _returnvalue_2)
  (`KismetSystemLibrary.PrintString` (`KismetStringLibrary.Concat_StrStr` "Playing new atmo: " (`KismetSystemLibrary.GetDisplayName` null)))
  (return false))

(fn `UserConstructionScript`)