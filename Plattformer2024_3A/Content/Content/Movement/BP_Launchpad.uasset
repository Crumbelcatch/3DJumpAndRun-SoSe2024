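; BP_Launchpad is a launch pad that propels the player along the pad mesh's up vector with a set force.
; Overlapping the collider sends a launch message to a Player-tagged actor, gated on a Falling check whose movement component lookup is missing.
; When flagged as trigger-activated, it starts with collision disabled until TriggerReciever enables it.
; Both paths set the mesh visible, so the inactive pad is not hidden.
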(event `self.ReceiveBeginPlay`
  ;[1 1 1] Begin Play
  (if (`self.ActivatedByTrigger`)
    (`SceneComponent.SetHiddenInGame` (`self.PadMesh`) false false)
    (`PrimitiveComponent.SetCollisionEnabled` (`self.Collider`) "NoCollision")
    (`PrimitiveComponent.SetCollisionEnabled` (`self.PadMesh`) "NoCollision")))

(event `/Game/Content/Trigger/BPI_TriggerReciever.Trigger Reciever`
  (params (`Triggers once` :type Boolean))
  ;[1 1 1] Enable Collision Switch
  (switch `ECollisionEnabled` (`PrimitiveComponent.GetCollisionEnabled` (`self.Collider`))
    (:`NoCollision`
      (`SceneComponent.SetHiddenInGame` (`self.PadMesh`) false false)
      (`PrimitiveComponent.SetCollisionEnabled` (`self.Collider`) "QueryOnly")
      (`PrimitiveComponent.SetCollisionEnabled` (`self.PadMesh`) "QueryAndPhysics"))))

(event `self.Collider.OnComponentBeginOverlap`
  (params (OverlappedComponent :type "PrimitiveComponent Object Reference") (OtherActor :type "Actor Object Reference") (OtherComp :type "PrimitiveComponent Object Reference") (OtherBodyIndex :type Integer) (bFromSweep :type Boolean) (SweepResult :type "HitResult Structure (by ref)"))
  ;[1 1 1] On Collide
  (if (`self.ActorHasTag` OtherActor "Player")
    (switch `EMovementMode` "MOVE_Falling" ; MISSING! \nGet Character Movement Component
      (:`MOVE_Falling`
        (message `/Game/Characters/Player/BPI_PlayerManipulation.LaunchPlayer` OtherActor (`self.LaunchForce`) (`SceneComponent.GetUpVector` (`self.PadMesh`)))))))

(fn `UserConstructionScript`)