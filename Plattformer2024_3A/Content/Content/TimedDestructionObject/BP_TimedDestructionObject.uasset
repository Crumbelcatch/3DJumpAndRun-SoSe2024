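; A timed platform actor intended to fall and fade after a tagged Player overlaps its trigger box.
; The overlap starts a timer on PlatformFall, but that event is empty and nothing here calls TogglePlatform.
; TogglePlatform plays or reverses a timeline that lowers the platform along its up vector while fading the Color alpha on a construction-time dynamic material instance.
; The collision toggle by timeline direction is unconnected, so it never runs.
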(event `self.ReceiveBeginPlay`
  ;[0.2066 1 0.4102] BeginPlay
  (bind _returnvalue (`MaterialInstanceDynamic.K2_GetVectorParameterValue` (`self.DMI Platform`) "Color"))
  (set `self.BaseColor` _returnvalue)
  (set `self.Platform starting Location` (`SceneComponent.K2_GetComponentLocation` (`self.Platform`))))

(event `self.Box.OnComponentBeginOverlap`
  (params (OverlappedComponent :type "PrimitiveComponent Object Reference") (OtherActor :type "Actor Object Reference") (OtherComp :type "PrimitiveComponent Object Reference") (OtherBodyIndex :type Integer) (bFromSweep :type Boolean) (SweepResult :type "HitResult Structure (by ref)"))
  (if (`ActorComponent.ComponentHasTag` OverlappedComponent "Player")
    (`KismetSystemLibrary.PrintString` "reached")
    (`KismetSystemLibrary.K2_SetTimerDelegate` (delegate `PlatformFall`) (`self.TimeTillFall`))))

(event `PlatformFall`)

(event `TogglePlatform`
  (params (bHide :type Boolean))
  (bind (_basecolor_r _basecolor_g _basecolor_b) (break `LinearColor` (`self.BaseColor`)))
  (if bHide
    (`KismetSystemLibrary.PrintString` "Toggle platform reached")
    (bind (_direction _alpha0_1) (`Timeline|PlatformFade` :!label _label)
      (:`Update`
        (`SceneComponent.K2_SetWorldLocation` (`self.Platform`) (`KismetMathLibrary.VLerp` (`self.Platform starting Location`) (- (`self.Platform starting Location`) (* (`SceneComponent.GetUpVector` (`self.Platform`)) (`self.FallDistance`))) _alpha0_1) false false)
        (`MaterialInstanceDynamic.SetVectorParameterValue` (`self.DMI Platform`) "Color" (make `LinearColor` _basecolor_r _basecolor_g _basecolor_b (- 1.0 _alpha0_1)))))
    (else
      (goto _label :!via `ReverseFromEnd`))))

(fn `UserConstructionScript`
  (bind _returnvalue (`PrimitiveComponent.CreateDynamicMaterialInstance` (`self.Platform`) 0 (`PrimitiveComponent.GetMaterial` (`self.Platform`) 0) "None"))
  (set `self.DMI Platform` _returnvalue))