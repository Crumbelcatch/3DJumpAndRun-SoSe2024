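; BP_MovingObject is a triggered actor that moves its mesh between its starting world position and a TargetLocation component.
; TriggerReciever drives the ObjectMoveAlpha timeline at a configurable rate, lerping position without sweep and choosing play or reverse from ObjectDataLocation.
; A DoOnce gates triggers and resets for repeatable moves unless TriggersOnce is set.
; Both finish directions set ObjectDataLocation false, and nothing here sets it true.
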(event `self.ReceiveBeginPlay`
  ;[0.531 1 0.4125] Begin Play
  (set `self.ObjectStartLocation` (`SceneComponent.K2_GetComponentLocation` (`self.Mesh`)))
  (`TimelineComponent.SetPlayRate` (`self.Object Move Alpha`) (`self.Object Move Rate`)))

(event `/Game/Content/Trigger/BPI_TriggerReciever.Trigger Reciever`
  (params (`Triggers once` :type Boolean))
  ;[1 0.1923 0.9016] Timeline for Move
  (set `self.Triggers Once` `Triggers once`)
  (`|ExecutionSequence`
    (:`then_0`
      (if (and (not (`self.Triggers Once`)) (`self.Object Data Location`))
        (`self.ResetMovementDoOnce`)))
    (:`then_1`
      (`/Engine/EditorBlueprintResources/StandardMacros.DoOnce` false :!label _label
        (:`Completed`
          (if (not (`self.Object Data Location`))
            (bind (_direction _alpha_0_1) (`Timeline|Object Move Alpha` :!label _label_2)
              (:`Update`
                (`SceneComponent.K2_SetWorldLocation` (`self.Mesh`) (`KismetMathLibrary.VLerp` (`self.ObjectStartLocation`) (`SceneComponent.K2_GetComponentLocation` (`self.Target Location`)) _alpha_0_1) false false))
              (:`Finished`
                ;[1 1 1] Object Move Finished
                (switch `ETimelineDirection` _direction
                  (:`Forward`
                    (set `self.Object Data Location` false))
                  (:`Backward`
                    (set `self.Object Data Location` false)))
                (if (not (`self.Triggers Once`))
                  (`self.ResetMovementDoOnce`))))
            (else
              (goto _label_2 :!via `Reverse`))))))))

(event `ResetMovementDoOnce`
  ;[1 0.1923 0.9016] Timeline for Move
  (goto _label :!via `Reset`))

(fn `UserConstructionScript`)