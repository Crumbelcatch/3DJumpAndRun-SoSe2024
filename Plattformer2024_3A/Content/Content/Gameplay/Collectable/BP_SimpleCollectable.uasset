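; BP_SimpleCollectable is a coin pickup that registers itself with the game mode on BeginPlay and spins at a random yaw rate.
; An overlap of its sphere by a Player-tagged actor notifies the game mode of collection and toggles the pickup inactive.
; ToggleCollectable switches sphere collision between query-only and none, but sets the coin visible in both branches, so collected coins are not hidden here.
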(event `self.ReceiveBeginPlay`
  ;[0.4327 1 0.3558] Begin Play
  (message `/Game/Characters/Player/BPI_Collectables.RegisterNewCollectable` (`GameplayStatics.GetGameMode`) self)
  (set `RotatingMovementComponent.RotationRate` (`KismetMathLibrary.MakeRotator` 0.0 0.0 (`KismetMathLibrary.RandomFloatInRange` 140.0 180.0)) (`self.RotatingMovement`)))

(event `self.Sphere.OnComponentBeginOverlap`
  (params (OverlappedComponent :type "PrimitiveComponent Object Reference") (OtherActor :type "Actor Object Reference") (OtherComp :type "PrimitiveComponent Object Reference") (OtherBodyIndex :type Integer) (bFromSweep :type Boolean) (SweepResult :type "HitResult Structure (by ref)"))
  ;[1 1 1] Collect Collectable
  (if (`self.ActorHasTag` OtherActor "Player")
    (message `/Game/Characters/Player/BPI_Collectables.Collected` (`GameplayStatics.GetGameMode`) self)
    (`self.Toggle Collectable` false)))

(event `Toggle Collectable`
  (params (Active :type Boolean))
  ;[1 1 1] Toggle Collectable
  (if Active
    (`SceneComponent.SetHiddenInGame` (`self.Coin`) false false)
    (`PrimitiveComponent.SetCollisionEnabled` (`self.Sphere`) "QueryOnly")
    (else
      (`SceneComponent.SetHiddenInGame` (`self.Coin`) false false)
      (`PrimitiveComponent.SetCollisionEnabled` (`self.Sphere`) "NoCollision"))))

(fn `UserConstructionScript`)