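; BP_Checkpoint is a checkpoint actor that holds a label and a respawn transform in its CheckpointData struct.
; On BeginPlay it writes Lable and the world transform of its RespawnTransform component into that struct.
; The construction script sets the CheckpointLabel text from Lable, so the label updates whenever the actor is constructed.
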(event `self.ReceiveBeginPlay`
  (bind _structout (setmembers `/Game/Content/Gameplay/Checkpoints/Struct_CheckpointData` :`StructRef` (`self.CheckpointData`) :`CheckpointLable` (`self.Lable`) :`CheckpointRespawn` (`SceneComponent.K2_GetComponentToWorld` (`self.RespawnTransform`))))
  (set `self.CheckpointData` _structout))

(fn `UserConstructionScript`
  (`TextRenderComponent.K2_SetText` (`self.CheckpointLabel`) (`KismetTextLibrary.Conv_StringToText` (`self.Lable`))))