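; Game instance for a platformer that handles level changes and tracks whether the player is using a gamepad.
; ChangeLevel maps a level selection to the main menu or the main ingame level and opens it by object reference.
; SwitchUsingGamepad stores the gamepad flag and forwards it to the game mode through SwitchInputModeMessage, while GetIsUsingGamepad exposes it.
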(event `self.ReceiveInit`)

(fn `ChangeLevel`
  (params (LevelToChangeTo :type "/Game/Maps/Enum_Level Enum" :default "NewEnumerator0"))
  (returns (Return :type Boolean))
  (switch `/Game/Maps/Enum_Level` LevelToChangeTo
    (:`NewEnumerator0`
      (`GameplayStatics.OpenLevelBySoftObjectPtr` "/Game/Maps/MainMenu.MainMenu")
      (return false))
    (:`NewEnumerator1`
      (`GameplayStatics.OpenLevelBySoftObjectPtr` "/Game/Maps/Main.Main")
      (return false))))

(fn `GetIsUsingGamepad`
  (returns (bIsUsingGamepad :type Boolean))
  (return (`self.bPlayerIsUsingGamepad`)))

(fn `SwitchUsingGamepad`
  (params (bUsingGamepad :type Boolean))
  (returns (Return :type Boolean))
  (bind _output_get (set `self.bPlayerIsUsingGamepad` bUsingGamepad))
  (message `/Game/Core/BPI_GameMode.SwitchInputMode` (`GameplayStatics.GetGameMode`) _output_get)
  (return false))