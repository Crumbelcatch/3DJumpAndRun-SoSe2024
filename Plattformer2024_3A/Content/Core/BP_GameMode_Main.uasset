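; Main game mode that acts as the hub for collectables, checkpoint respawns, level sequence cinematics and UI.
; Registered collectables map to collected flags, with count changes sent to counter widgets through messages.
; Respawn ports the player to the last checkpoint and resets that checkpoint's collected items, or requests a level change if none is saved.
; It also manages countdown, tutorial, pause and cheat widgets, input modes, and a tag-located sound manager reference.
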(event `self.ReceiveBeginPlay`
  ;[0.3269 1 0.3191] Begin play
  (`WidgetBlueprintLibrary.SetInputMode_GameOnly` (`GameplayStatics.GetPlayerController` 0))
  (set `self.CollectedCollectables` 0)
  (set `self.LastCheckpoint` (make `/Game/Gameplay/Checkpoints/Struct_CheckpointData` "" (`KismetMathLibrary.MakeTransform` (0.0 0.0 0.0))))
  ;[1 1 1] Get Sound Manager
  (bind _outactors (`GameplayStatics.GetAllActorsOfClassWithTag` "/Script/Engine.Actor" "SoundManager"))
  (bind _output (`|GetArrayItem` _outactors))
  (`/Engine/EditorBlueprintResources/StandardMacros.IsValid` _output
    (:`Is Valid`
      (set `self.SoundManagerRef` _output))
    (:`Is Not Valid`
      (`KismetSystemLibrary.PrintString` "Sound Manager Not Found In Level!"))))

(fn `CinematicEnd`
  (returns (Return :type Boolean))
  (`|ExecutionSequence`
    (:`then_0`
      (`self.EnableInput` (`GameplayStatics.GetPlayerCharacter` 0) (`GameplayStatics.GetPlayerController` 0)))
    (:`then_1`
      (`SkeletalMeshComponent.SetAnimationMode` (`Character.Mesh` (`GameplayStatics.GetPlayerCharacter` 0)) "AnimationBlueprint" true))
    (:`then_2`
      (`/Engine/EditorBlueprintResources/StandardMacros.IsValid` (`self.CurrentSequencePlayer`)
        (:`Is Valid`
          (`self.K2_DestroyActor` (`self.CurrentSequencePlayer`)))))
    (:`then_3`
      ;[1 0.4584 0.05728] return
      (return false))))

(fn `Collected`
  (params (CollectableRef :type "Actor Object Reference"))
  (returns (Return :type Boolean))
  (locals (LCollectable :type "Actor Object Reference"))
  (set `local.LCollectable` CollectableRef)
  (`|ExecutionSequence`
    (:`then_0`
      (`/Engine/EditorBlueprintResources/StandardMacros.IncrementInt` (`self.CollectedCollectables`)))
    (:`then_1`
      (if (`.ReturnValue` (`BlueprintMapLibrary.Map_Find` (`self.CollectableRefs`) (`local.LCollectable`)))
        (`BlueprintMapLibrary.Map_Add` (`self.CollectableRefs`) (`local.LCollectable`) true)))
    (:`then_2`
      (for _array_element (`self.CounterWidgetRefs`)
        (message `/Game/Gameplay/Collectables/BPI_Collectables.Collected` _array_element (`local.LCollectable`))))
    (:`then_3`
      ;[1 0.5239 0.1351] return
      (return false))))

(fn `GetCollectedCollectables`
  (returns (CollectedCollectables :type Integer))
  (return (`self.CollectedCollectables`)))

(fn `GetSoundManagerRef`
  (returns (SoundManager :type "Actor Object Reference"))
  (return (`self.SoundManagerRef`)))

(fn `RegisterNewCollectable`
  (params (NewCollectable :type "Actor Object Reference"))
  (returns (Return :type Boolean))
  (`BlueprintMapLibrary.Map_Add` (`self.CollectableRefs`) NewCollectable)
  (return false))

(fn `RegisterNewCounter`
  (params (NewCounter :type "UserWidget Object Reference"))
  (returns (Return :type Boolean))
  (`KismetArrayLibrary.Array_Add` (`self.CounterWidgetRefs`) NewCounter)
  (return false))

(fn `RespawnCollectable`
  (returns (Return :type Boolean))
  (return false))

(fn `RespawnCollectablesIfCollected`
  (params (Collectables :type "Array of Actor Object Reference"))
  (locals (LCurrentCollectable :type "Actor Object Reference"))
  (bind (_value _returnvalue) (`BlueprintMapLibrary.Map_Find` (`self.CollectableRefs`) (`local.LCurrentCollectable`)))
  (for _array_element Collectables
    (bind _output_get (set `local.LCurrentCollectable` _array_element))
    (`/Engine/EditorBlueprintResources/StandardMacros.IsValid` _output_get
      (:`Is Valid`
        (if (and _value _returnvalue)
          (`|ExecutionSequence`
            (:`then_0`
              (message `/Game/Gameplay/Collectables/BPI_Collectables.RespawnCollectable` (`local.LCurrentCollectable`)))
            (:`then_1`
              (`/Engine/EditorBlueprintResources/StandardMacros.DecrementInt` (`self.CollectedCollectables`)))
            (:`then_2`
              (for _array_element_2 (`self.CounterWidgetRefs`)
                (message `/Game/Gameplay/Collectables/BPI_Collectables.RespawnCollectable` _array_element_2)))
            (:`then_3`
              (`BlueprintMapLibrary.Map_Add` (`self.CollectableRefs`) (`local.LCurrentCollectable`))))))))
  ;[1 0.4897 0.1588] return
  (return))

(fn `RespawnPlayer`
  (returns (Return :type Boolean))
  (bind (_checkpointlabel _checkpointrespawntransform _collectables) (break `/Game/Gameplay/Checkpoints/Struct_CheckpointData` (`self.LastCheckpoint`)))
  (if (== (.location (`.CheckpointRespawnTransform_5_45F4D3E448D53A9C5DDE9B94B68BF015` (break `/Game/Gameplay/Checkpoints/Struct_CheckpointData` (`self.LastCheckpoint`)))) (0.0 0.0 0.0))
    (message `/Game/Core/BPI_GameInstance.ChangeLevel` (`GameplayStatics.GetGameInstance`) (`KismetMathLibrary.Conv_ByteToInt` 1))
    (return false)
    (else
      (message `/Game/Characters/Player/BPI_PlayerManipulation.PortPlayerToTransform` (`GameplayStatics.GetPlayerCharacter` 0) _checkpointrespawntransform)
      (bind _movementcomponentref (message `/Game/Characters/Player/BPI_PlayerValues.GetCharacterMovementComponent` (`GameplayStatics.GetPlayerCharacter` 0)))
      (set `MovementComponent.Velocity` (0.0 0.0 0.0) _movementcomponentref)
      (`self.RespawnCollectablesIfCollected` _collectables)
      (return false))))

(fn `SaveNewCheckpoint`
  (params (CheckpointData :type "/Game/Gameplay/Checkpoints/Struct_CheckpointData Structure"))
  (returns (Return :type Boolean))
  (bind _output_get (set `self.LastCheckpoint` CheckpointData))
  (bind (_checkpointlabel _checkpointrespawntransform) (break `/Game/Gameplay/Checkpoints/Struct_CheckpointData` _output_get))
  (`KismetSystemLibrary.PrintString` (`KismetStringLibrary.Concat_StrStr` "New checkpoint saved: " _checkpointlabel (`KismetStringLibrary.Conv_TransformToString` _checkpointrespawntransform)))
  (return false))

(fn `ShowHideGlobalCountdown`
  (params (CountdownValue :type "Float (double-precision)") (bShow :type Boolean))
  (returns (Return :type Boolean))
  (locals (LCDValue :type "Float (double-precision)" :default 0.0))
  (set `local.LCDValue` CountdownValue)
  (if bShow
    (`|ExecutionSequence`
      (:`then_0`
        ;[0 0 0] remove possibly existing countdown widget
        (`/Engine/EditorBlueprintResources/StandardMacros.IsValid` (`self.VisibleDountdownWidgetRef`)
          (:`Is Valid`
            (`/Game/UI/Gameplay/WBP_Countdown.DestroyWidget` (`self.VisibleDountdownWidgetRef`))
            (set `self.VisibleDountdownWidgetRef` null))))
      (:`then_1`
        ;[0 0 0] create new countdown widget and show on viewport
        (bind _returnvalue (`|CreateWidget` "/Game/UI/Gameplay/WBP_Countdown.WBP_Countdown_C" null (`local.LCDValue`)))
        (bind _output_get (set `self.VisibleDountdownWidgetRef` _returnvalue))
        (`UserWidget.AddToViewport` _output_get 0))
      (:`then_2`
        ;[1 0.2647 0.0675] return
        (return true)))
    (else
      ;[1 1 1] Hide countdown
      (`/Engine/EditorBlueprintResources/StandardMacros.IsValid` (`self.VisibleDountdownWidgetRef`)
        (:`Is Valid`
          (`/Game/UI/Gameplay/WBP_Countdown.DestroyWidget` (`self.VisibleDountdownWidgetRef`))
          (set `self.VisibleDountdownWidgetRef` null)
          ;[1 0.2647 0.0675] return
          (return true))))))

(fn `ShowHideTutorialTextbox`
  (params (TutorialText :type Text) (bShow :type Boolean))
  (returns (return :type Boolean))
  (locals (TutorialTextContent :type Text))
  (set `local.TutorialTextContent` TutorialText)
  (if bShow
    (`|ExecutionSequence`
      (:`then_0`
        ;[0 0 0] remove possibly existing countdown widget
        (`/Engine/EditorBlueprintResources/StandardMacros.IsValid` (`self.VisibleTutorialWidgetRef`)
          (:`Is Valid`
            (`/Game/UI/Gameplay/WBP_Tutorial.DestroyWidget` (`self.VisibleTutorialWidgetRef`))
            (set `self.VisibleDountdownWidgetRef` null))))
      (:`then_1`
        ;[0 0 0] create new countdown widget and show on viewport
        (bind _returnvalue (`|CreateWidget` "/Game/UI/Gameplay/WBP_Tutorial.WBP_Tutorial_C" null (`local.TutorialTextContent`)))
        (bind _output_get (set `self.VisibleTutorialWidgetRef` _returnvalue))
        (`UserWidget.AddToViewport` _output_get 0))
      (:`then_2`
        ;[1 0.2647 0.0675] return
        (return true)))
    (else
      ;[1 1 1] Hide countdown
      (`/Engine/EditorBlueprintResources/StandardMacros.IsValid` (`self.VisibleTutorialWidgetRef`)
        (:`Is Valid`
          (`/Game/UI/Gameplay/WBP_Tutorial.DestroyWidget` (`self.VisibleTutorialWidgetRef`))
          (set `self.VisibleDountdownWidgetRef` null)
          ;[1 0.2647 0.0675] return
          (return true))))))

(fn `StartCinematic`
  (params (SequenceToPlay :type "LevelSequence Object Reference"))
  (returns (Return :type Boolean))
  (locals (LSequence :type "LevelSequence Object Reference"))
  (set `local.LSequence` SequenceToPlay)
  (`self.DisableInput` (`GameplayStatics.GetPlayerCharacter` 0) (`GameplayStatics.GetPlayerController` 0))
  (bind (_outactor _returnvalue) (`LevelSequencePlayer.CreateLevelSequencePlayer` (`local.LSequence`)))
  (set `self.CurrentSequencePlayer` _outactor)
  (`MovieSceneSequencePlayer.Play` _returnvalue)
  (return false))

(fn `SwitchInputMode`
  (params (bIsUsingGamepad :type Boolean))
  (returns (Return :type Boolean))
  (if bIsUsingGamepad
    (set `PlayerController.bShowMouseCursor` false (`GameplayStatics.GetPlayerController` 0))
    (`/Engine/EditorBlueprintResources/StandardMacros.IsValid` (`self.VisibleViewportWidgetRef`)
      (:`Is Valid`
        (message `/Game/UI/BPI_Widgets.SwitchFocusCheck` (`self.VisibleViewportWidgetRef`) true))
      (:`Is Not Valid`
        _))
    (return false)
    (else
      (`/Engine/EditorBlueprintResources/StandardMacros.IsValid` (`self.VisibleViewportWidgetRef`)
        (:`Is Valid`
          (set `PlayerController.bShowMouseCursor` true (`GameplayStatics.GetPlayerController` 0))
          (message `/Game/UI/BPI_Widgets.SwitchFocusCheck` (`self.VisibleViewportWidgetRef`) false))
        (:`Is Not Valid`
          _))
      (return false))))

(fn `ToggleCheatUI`
  (returns (Return :type Boolean))
  (if (not (`self.bCheatUIActive`))
    (`|ExecutionSequence`
      (:`then_0`
        (`/Engine/EditorBlueprintResources/StandardMacros.IsValid` (`self.CheatUIRef`)
          (:`Is Not Valid`
            (bind _returnvalue (`|CreateWidget` "/Game/UI/Debug/WBP_CheatMenu.WBP_CheatMenu_C"))
            (set `self.CheatUIRef` _returnvalue))))
      (:`then_1`
        (`UserWidget.AddToViewport` (`self.CheatUIRef`) 0))
      (:`then_2`
        (`WidgetBlueprintLibrary.SetInputMode_GameAndUIEx` (`GameplayStatics.GetPlayerController` 0) (`self.CheatUIRef`))
        (set `PlayerController.bShowMouseCursor` true (`GameplayStatics.GetPlayerController` 0)))
      (:`then_3`
        (set `self.bCheatUIActive` true)
        ;[1 0.4278 0.1332] return
        (return false)))
    (else
      (`Widget.RemoveFromParent` (`self.CheatUIRef`))
      (`WidgetBlueprintLibrary.SetInputMode_GameOnly` (`GameplayStatics.GetPlayerController` 0))
      (set `PlayerController.bShowMouseCursor` false (`GameplayStatics.GetPlayerController` 0))
      (set `self.bCheatUIActive` false)
      ;[1 0.441 0.1462] return
      (return false))))

(fn `TogglePause`
  (returns (Return :type Boolean))
  (`|ExecutionSequence`
    (:`then_0`
      ;[1 1 1] Menu widget
      (if (not (`self.bIsGamePaused`))
        (`/Engine/EditorBlueprintResources/StandardMacros.IsValid` (`self.PauseMenuRef`)
          (:`Is Valid`
            (message `/Game/UI/BPI_Widgets.RemoveWidget` (`self.PauseMenuRef`) false))
          (:`Is Not Valid`
            _))
        (bind _returnvalue (`|CreateWidget` "/Game/UI/Gameplay/WBP_PauseMenu.WBP_PauseMenu_C"))
        (bind _output_get (set `self.PauseMenuRef` _returnvalue))
        (set `self.VisibleViewportWidgetRef` _output_get)
        (`UserWidget.AddToViewport` (`self.PauseMenuRef`) 0)
        (else
          (`/Engine/EditorBlueprintResources/StandardMacros.IsValid` (`self.PauseMenuRef`)
            (:`Is Valid`
              (message `/Game/UI/BPI_Widgets.RemoveWidget` (`self.PauseMenuRef`) true)
              (set `self.VisibleViewportWidgetRef` null))))))
    (:`then_1`
      ;[1 1 1] Input
      (if (not (`self.bIsGamePaused`))
        (`WidgetBlueprintLibrary.SetInputMode_GameAndUIEx` (`GameplayStatics.GetPlayerController` 0) (`self.PauseMenuRef`))
        (bind _bisusinggamepad (message `/Game/Core/BPI_GameInstance.GetIsUsingGamepad` (`GameplayStatics.GetGameInstance`)))
        (if (not _bisusinggamepad)
          (set `PlayerController.bShowMouseCursor` true (`GameplayStatics.GetPlayerController` 0)))
        (else
          (`WidgetBlueprintLibrary.SetInputMode_GameOnly` (`GameplayStatics.GetPlayerController` 0))
          (set `PlayerController.bShowMouseCursor` false (`GameplayStatics.GetPlayerController` 0)))))
    (:`then_2`
      ;[1 1 1] Game state
      (`GameplayStatics.SetGamePaused` (not (`self.bIsGamePaused`)))
      (set `self.bIsGamePaused` (not (`self.bIsGamePaused`))))
    (:`then_3`
      ;[1 0.5435 0.1754] return
      (return false))))

(fn `UserConstructionScript`)